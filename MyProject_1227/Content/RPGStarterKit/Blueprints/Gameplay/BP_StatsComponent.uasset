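; Actor component for the RPG starter kit that stores a list of name/value stats, with lookups by index and increases by index or name.
; Each increase runs StatHasChanged, which branches on stat name for custom behavior, then fires StatChanged for UI updates.
; Experience changes trigger a fixed-threshold level-up check that assumes Level and Experience occupy indices 0 and 1.
; Increasing by index writes an empty name, bypassing that check.
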(event EventTick
  (params (DeltaSeconds :type Float%20%28single-precision%29)))

(event EventInitializeComponent)

(fn IncreaseStatbyIndex
  (params (Index :type Integer :default 0) (Value :type Integer :default 0))
  (bind _statslist (Variables|Default|GetStatsList))
  (bind _item (Utilities|Array|Get(acopy) _statslist Index))
  (bind _statvalue (Utilities|Struct|BreakBPS_SingleStat _item))
  (bind _returnvalue (+ Value _statvalue))
  (bind _bps_singlestat (Utilities|Struct|MakeBPS_SingleStat "" _returnvalue))
  ;[1 1 1] Increase the value of the specified stat
  (Utilities|Array|SetArrayElem (Variables|Default|GetStatsList) Index _bps_singlestat)
  (CallFunction|StatHasChanged _bps_singlestat))

(fn GetValuebyIndex
  (params (Index :type Integer :default 0))
  ;[1 1 1] Return the value from the array specified by the supplied index
  (return (.StatValue (Utilities|Struct|BreakBPS_SingleStat (Utilities|Array|Get(acopy) (Variables|Default|GetStatsList) Index)))))

(fn GetNamebyIndex
  (params (Integer :type Integer :default 0))
  ;[1 1 1] Return the name of the stat from the array specified by the supplied index
  (return (.StatName (Utilities|Struct|BreakBPS_SingleStat (Utilities|Array|Get(acopy) (Variables|Default|GetStatsList) Integer)))))

(fn GetStatObjectbyIndex
  (params (Index :type Integer :default 0))
  ;[1 1 1] Return the actual stat object from the array specified by the supplied index
  (return (Utilities|Array|Get(acopy) (Variables|Default|GetStatsList) Index)))

(fn IncreaseStatbyName
  (params (StatName :type Text) (Value :type Integer :default 0))
  ;[1 1 1] Cache stat name
  (LocalVariables|SetCurrentStatName StatName)
  ;[1 1 1] If the specified stat is in the list...
  (for (_array_element _array_index) (Variables|Default|GetStatsList)
    (if (Utilities|Enum|Equal(Enum) (.StatName (Utilities|Struct|BreakBPS_SingleStat _array_element)) (LocalVariables|GetCurrentStatName))
      ;[1 1 1] ... increase the value and save it
      (Utilities|Array|SetArrayElem (Variables|Default|GetStatsList) _array_index (Utilities|Struct|MakeBPS_SingleStat (LocalVariables|GetCurrentStatName) (+ (.StatValue (Utilities|Struct|BreakBPS_SingleStat _array_element)) Value)))
      (CallFunction|StatHasChanged (Utilities|Struct|MakeBPS_SingleStat (LocalVariables|GetCurrentStatName) (+ (.StatValue (Utilities|Struct|BreakBPS_SingleStat _array_element)) Value))))))

(fn GetAllStats
  ;[1 1 1] Return the array of stats
  (return (Variables|Default|GetStatsList)))

(fn CheckXPforLevelUp
  (bind _statslist (Variables|Default|GetStatsList))
  (bind _item (Utilities|Array|Get(acopy) _statslist))
  (bind _item_2 (Utilities|Array|Get(acopy) _statslist 1))
  (bind (_statname _statvalue) (Utilities|Struct|BreakBPS_SingleStat _item_2))
  (bind (_statname_2 _statvalue_2) (Utilities|Struct|BreakBPS_SingleStat _item))
  ;[1 0.29 0.29] Attention: This only functions correctly when stat index 0 is Level and index 1 Experience!
  (if (>= _statvalue 200)
    ;[1 1 1] Increase level
    (Utilities|Array|SetArrayElem (Variables|Default|GetStatsList) 0 (Utilities|Struct|MakeBPS_SingleStat _statname_2 (+ _statvalue_2 1)))
    ;[1 1 1] Set new XP value
    (Utilities|Array|SetArrayElem (Variables|Default|GetStatsList) 1 (Utilities|Struct|MakeBPS_SingleStat _statname (- _statvalue 200)))))

(fn StatHasChanged
  (params (Stat :type BPS%20Single%20Stat%20Structure))
  (Utilities|FlowControl|Sequence
    (:then_0
      ;[1 1 1] Implement custom behaviour for certain stats here
      (switch string (Utilities|String|ToString(Text) (.StatName (Utilities|Struct|BreakBPS_SingleStat Stat)))
        (:Experience
          (CallFunction|CheckXPforLevelUp))))
    (:then_1
      ;[1 1 1] Allows to update UI
      (Default|CallStatChanged))))