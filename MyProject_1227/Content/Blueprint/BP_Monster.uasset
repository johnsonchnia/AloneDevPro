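; BP_Monster is an AI monster character that initializes from a character info value on BeginPlay and tracks its own health.
; AnyDamage subtracts incoming damage from AIZZHealth and does nothing further.
; An unconnected chain, which never runs, would update the widget health bar and, at zero health or below, set the "isdead" blackboard key, stop movement and play a death animation once.
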(event `self.ReceiveTick`
  (params (DeltaSeconds :type "Float (single-precision)"))
  (`parent.ReceiveTick` 0.0))

(event `self.ReceiveBeginPlay`
  (`self.InitCharacter` (`self.ChacterInfo`)))

(event `self.ReceiveAnyDamage`
  (params (Damage :type "Float (single-precision)") (DamageType :type "DamageType Object Reference") (InstigatedBy :type "Controller Object Reference") (DamageCauser :type "Actor Object Reference"))
  (set `self.AI_ZZ_Health` (- (`self.AI_ZZ_Health`) Damage)))

(fn `UserConstructionScript`)