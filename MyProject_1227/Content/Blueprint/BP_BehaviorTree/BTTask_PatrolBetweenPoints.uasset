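; Behavior Tree task that keeps an enemy AI walking a looping route of patrol points taken from its EnemyController.
; Execution caches the controller and points, then opens a gate that lets Tick drive AI MoveTo toward the current point.
; Each successful move advances the index, wrapping to the first point.
; A valid Target or HasInvestigateLocation on the Blackboard finishes the task successfully and closes the gate.
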(event `self.ReceiveTick`
  (params (OwnerActor :type "Actor Object Reference") (DeltaSeconds :type "Float (single-precision)"))
  ;[1 1 1] 開始執行任務并繼續運行它，直到它完成
  (`/Engine/EditorBlueprintResources/StandardMacros.Gate` true :!label _label
    (:`Exit`
      ;[1 1 1] 當AI有目標時，中斷巡邏
      (if (`KismetSystemLibrary.IsValid` (`BTFunctionLibrary.GetBlackboardValueAsObject` (`self.Target`)))
        ;[1 1 1] 結束這次任務
        (`self.FinishExecute` true :!label _label_2)
        (`self.CloseGate`)
        (else
          ;[1 1 1] 當AI聽到什麽，中斷
          (if (`BTFunctionLibrary.GetBlackboardValueAsBool` (`self.HasInvestigateLocation`))
            (goto _label_2)
            (else
              ;[1 1 1] 當AI達到攻擊範圍時停止
              (`|AIMoveTo` (`Controller.K2_GetPawn` (`self.EnemyController`)) (`KismetArrayLibrary.Array_Get` (`self.PatrolPoints`) (`self.CurrentPatrolIndex`)) null 50.0
                (:`OnSuccess`
                  (set `self.CurrentPatrolIndex` (+ (`self.CurrentPatrolIndex`) 1))
                  ;[1 1 1] 如果達到最後一個點則重置巡邏點
                  (if (>= (`self.CurrentPatrolIndex`) (`KismetArrayLibrary.Array_Length` (`self.PatrolPoints`)))
                    (set `self.CurrentPatrolIndex` 0)))))))))))

(event `self.ReceiveExecute`
  (params (OwnerActor :type "Actor Object Reference"))
  ;[1 1 1] 開始執行任務并繼續運行它，直到它完成
  (bind _asenemy_controller (cast `/Game/Blueprint/EnemyController` OwnerActor))
  (set `self.PatrolPoints` (`/Game/Blueprint/EnemyController.PatrolPoints` _asenemy_controller))
  (set `self.EnemyController` _asenemy_controller)
  (goto _label :!via `Open`))

(event `CloseGate`
  ;[1 1 1] 開始執行任務并繼續運行它，直到它完成
  (goto _label :!via `Close`))