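; Behavior tree task that makes an AI chase its blackboard target until within attack range or a time limit runs out.
; Execution resets the timer, caches the EnemyController and opens a gate that lets Tick reissue AIMoveTo toward the target's location, using the controller's attack range as acceptance radius.
; Reaching range finishes successfully; exceeding MaximumChaseTime resets the target and also finishes successfully, closing the gate.
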(event `self.ReceiveTick`
  (params (OwnerActor :type "Actor Object Reference") (DeltaSeconds :type "Float (single-precision)"))
  (bind _enemycontroller (`self.EnemyController`))
  ;[1 1 1] 開始執行任務并繼續運行它，直到它完成
  (set `self.Timer` (+ DeltaSeconds (`self.Timer`)))
  (`/Engine/EditorBlueprintResources/StandardMacros.Gate` true :!label _label
    (:`Exit`
      ;[1 1 1] 檢查追逐時間
      (if (>= (`self.Timer`) (`self.MaximumChaseTime`))
        ;[1 1 1] 如果時間超過，重置目標
        (`/Game/Blueprint/EnemyController.ResetTarget` _enemycontroller)
        (else
          ;[1 1 1] 當AI達到攻擊範圍時停止追逐
          (`|AIMoveTo` (`Controller.K2_GetPawn` _enemycontroller) (`Actor.K2_GetActorLocation` (`BTFunctionLibrary.GetBlackboardValueAsActor` (`self.Target`))) null (`/Game/Blueprint/EnemyController.AttackRangeValue` (stale `self.ReceiveExecute` _asenemy_controller))
            (:`OnSuccess`
              _))))
      ;[1 1 1] 結束任務
      (`self.FinishExecute` true)
      (`self.CloseGate`))))

(event `self.ReceiveExecute`
  (params (OwnerActor :type "Actor Object Reference"))
  ;[1 1 1] 開始執行任務并繼續運行它，直到它完成
  (set `self.Timer` 0.0) ; Reset timer
  (bind _asenemy_controller (cast `/Game/Blueprint/EnemyController` OwnerActor))
  (set `self.EnemyController` _asenemy_controller)
  (goto _label :!via `Open`))

(event `CloseGate`
  ;[1 1 1] 開始執行任務并繼續運行它，直到它完成
  (goto _label :!via `Close`))