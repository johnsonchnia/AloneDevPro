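; Behavior tree task that sends an enemy AI pawn to investigate a location stored in the blackboard.
; Execution caches the EnemyController and opens a gate, so Tick repeatedly checks for an attack target and otherwise moves the pawn toward the target location.
; Spotting a target or reaching the location clears the investigate flag, finishes with success and closes the gate.
; A failed move has no handler.
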(event `self.ReceiveTick`
  (params (OwnerActor :type "Actor Object Reference") (DeltaSeconds :type "Float (single-precision)"))
  ;[1 1 1] 開始執行任務并繼續運行它，直到它完成
  (`/Engine/EditorBlueprintResources/StandardMacros.Gate` true :!label _label
    (:`Exit`
      ;[1 1 1] 如果AI看見敵人，不要進一步調查
      (if (not (`KismetSystemLibrary.IsValid` (`BTFunctionLibrary.GetBlackboardValueAsObject` (`self.AttackTarget`))))
        ;[1 1 1] 移動以調查位置
        (`|AIMoveTo` (`Controller.K2_GetPawn` (`self.EnemyController`)) (`BTFunctionLibrary.GetBlackboardValueAsVector` (`self.Target`)) null 150.0
          (:`OnSuccess`
            _)))
      ;[1 1 1] 结束此任务并将调查位置设置为false
      (`BTFunctionLibrary.SetBlackboardValueAsBool` (`self.HasInvestigateLocation`))
      (`self.FinishExecute` true)
      (`self.CloseGate`))))

(event `self.ReceiveExecute`
  (params (OwnerActor :type "Actor Object Reference"))
  ;[1 1 1] 開始執行任務并繼續運行它，直到它完成
  (bind _asenemy_controller (cast `/Game/Blueprint/EnemyController` OwnerActor))
  (set `self.EnemyController` _asenemy_controller)
  (goto _label :!via `Open`))

(event `CloseGate`
  ;[1 1 1] 開始執行任務并繼續運行它，直到它完成
  (goto _label :!via `Close`))