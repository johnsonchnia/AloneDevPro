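; Behavior tree task that makes the AI-controlled StandardEnemy attack.
; ReceiveExecute caches the owner as an EnemyController and opens a gate that Tick passes through.
; On that tick it casts the controlled pawn to StandardEnemy, calls Attack, finishes successfully and closes the gate, so the attack fires once per execution.
; The direct cast is flagged in a comment as needing an interface instead.
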(event `self.ReceiveTick`
  (params (OwnerActor :type "Actor Object Reference") (DeltaSeconds :type "Float (single-precision)"))
  ;[1 1 1] 開始執行任務并繼續運行它，直到它完成
  (`/Engine/EditorBlueprintResources/StandardMacros.Gate` true :!label _label
    (:`Exit`
      ;[1 1 1] 使敵人產生攻擊
      (bind _asstandard_enemy (cast `/Game/Blueprint/StandardEnemy` (`Controller.K2_GetPawn` (`self.EnemyController`))))
      (`/Game/Blueprint/StandardEnemy.Attack` _asstandard_enemy) ; Should be interface!
      ;[1 1 1] 結束任務
      (`self.FinishExecute` true)
      (`self.CloseGate`))))

(event `self.ReceiveExecute`
  (params (OwnerActor :type "Actor Object Reference"))
  ;[1 1 1] 開始執行任務并繼續運行它，直到它完成
  (bind _asenemy_controller (cast `/Game/Blueprint/EnemyController` OwnerActor))
  (set `self.EnemyController` _asenemy_controller)
  (goto _label :!via `Open`))

(event `CloseGate`
  ;[1 1 1] 開始執行任務并繼續運行它，直到它完成
  (goto _label :!via `Close`))