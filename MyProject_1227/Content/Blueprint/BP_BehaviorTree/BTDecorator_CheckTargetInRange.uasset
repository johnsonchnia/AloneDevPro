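; Behavior tree decorator that passes when the AI's target is within attack range of the controlled pawn.
; It casts the owner to EnemyController, then compares the distance between the pawn and the blackboard Target actor to the blackboard AttackRange value.
; A fixed padding is added to the range before the comparison.
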(fn `PerformConditionCheckAI`
  (params (OwnerController :type "AIController Object Reference") (ControlledPawn :type "Pawn Object Reference"))
  (returns (ReturnValue :type Boolean))
  (bind _asenemy_controller (cast `/Game/Blueprint/EnemyController` OwnerController))
  (set `self.EnemyController` _asenemy_controller)
  (return (>= (+ (`BTFunctionLibrary.GetBlackboardValueAsFloat` (`self.AttackRange`)) 50.0) (`KismetMathLibrary.VSize` (- (`Actor.K2_GetActorLocation` (`BTFunctionLibrary.GetBlackboardValueAsActor` (`self.Target`))) (`Actor.K2_GetActorLocation` (`Controller.K2_GetPawn` (`self.EnemyController`))))))))