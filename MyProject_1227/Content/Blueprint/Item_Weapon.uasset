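; Weapon item Blueprint that extends a pickup parent, keeping its hit collision disabled until EquipWeapon enables it and switches off the pickup trigger.
; On weapon overlap, a short capsule trace estimates the impact location, which it passes with the overlapped actor to player 0's RPGCharacter through HitEnemyCharacter.
; StartTrails runs a socket-to-socket weapon trail after a given delay for a given duration.
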(event `self.ReceiveBeginPlay`
  (`parent.ReceiveBeginPlay`)
  ;[1 1 1] Disable weapon collision by default - only enable when picked up
  (`PrimitiveComponent.SetCollisionEnabled` (`self.WeaponCollision`) "NoCollision"))

(event `self.WeaponCollision.OnComponentBeginOverlap`
  (params (OverlappedComponent :type "PrimitiveComponent Object Reference") (OtherActor :type "Actor Object Reference") (OtherComp :type "PrimitiveComponent Object Reference") (OtherBodyIndex :type Integer) (bFromSweep :type Boolean) (SweepResult :type "HitResult Structure (by ref)"))
  (bind _returnvalue (`self.K2_GetActorLocation`))
  ;[1 1 1] Find out where the hit actually occured
  (bind _outhit (`KismetSystemLibrary.CapsuleTraceSingle_NEW` _returnvalue (+ _returnvalue (`self.GetActorForwardVector`)) 5.0 60.0 "TraceTypeQuery1"))
  ;[1 1 1] Let the player know that the weapon hit something
  (bind _asrpgcharacter (cast `/Game/Blueprint/RPGCharacter` (`GameplayStatics.GetPlayerCharacter` 0)))
  (`/Game/Blueprint/RPGCharacter.HitEnemyCharacter` _asrpgcharacter OtherActor (`.Location` (`GameplayStatics.BreakHitResult` _outhit))))

(event `StartTrails`
  (params (StartDelay :type "Float (double-precision)") (Duration :type "Float (double-precision)"))
  ;[1 1 1] Weapon Trails
  (`KismetSystemLibrary.Delay` StartDelay)
  (`ParticleSystemComponent.BeginTrails` "Emitter_Start" "Emitter_End" "ETrailWidthMode_FromSecond" 1.0)
  (`KismetSystemLibrary.Delay` Duration)
  (`ParticleSystemComponent.EndTrails`))

(event `EquipWeapon`
  ;[1 1 1] Enable Weapon collision when equipped
  (`self.SetActorEnableCollision` true)
  (`PrimitiveComponent.SetCollisionEnabled` (`self.WeaponCollision`) "QueryAndPhysics")
  (`PrimitiveComponent.SetCollisionEnabled` (`self.Trigger`) "NoCollision"))

(event `self.PickupItem_Event`
  ;[1 1 1] Implement custom behaviour for picksups here
  (`parent.PickupItem_Event`))

(fn `UserConstructionScript`
  (`parent.UserConstructionScript`))