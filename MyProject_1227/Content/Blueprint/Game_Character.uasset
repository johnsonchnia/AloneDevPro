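; Game character base that holds a CharacterInfo record and displays a floating health bar plus a HUD target panel.
; ShowBlood lazily creates and reuses a WB_Blood widget, which Tick refreshes and projects above the mesh bounds, moving it offscreen if projection fails.
; Clicking the mesh fills and shows the HUD target panel.
; GetBloodInfo supplies the bar data, but its name, health and magic struct node is unconnected.
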(event `self.ReceiveTick`
  (params (DeltaSeconds :type "Float (single-precision)"))
  (`self.UpdateBloodBar`))

(event `self.Mesh.OnClicked`
  (params (TouchedComponent :type "PrimitiveComponent Object Reference") (ButtonPressed :type "Key Structure" :default "AnyKey"))
  (`self.ShowCharacterInfo`))

(fn `GetCharacterInfo`
  (returns (CharacterInfo :type "/Game/Blueprint/DataStruct/S_CharacterInfo Structure"))
  (return (`self.CharacterInfo`)))

(fn `GetCharacterType`
  (returns (Type :type "/Game/Blueprint/DataStruct/E_CharacterType Enum"))
  (return (`.CharacterType_22_3DD4EC3F4D7B8C36460DDA8F19BEA29C` (break `/Game/Blueprint/DataStruct/S_CharacterInfo` (`self.CharacterInfo`)))))

(fn `HideBlood`
  (bind _wb_blood (`self.WB_Blood`))
  (`/Engine/EditorBlueprintResources/StandardMacros.IsValid` _wb_blood
    (:`Is Valid`
      (`Widget.SetVisibility` _wb_blood "Hidden")
      (set `self.IsBloodBarShowing` false))))

(fn `HideCharacterInfo`
  (`Widget.SetVisibility` (`/Game/UI/WB_Hud.WB_TargetActor` (`/Game/Blueprint/GameAPI_Lib.GetHudWidget`)) "Hidden"))

(fn `InitCharacter`
  (params (CharacterInfo :type "/Game/Blueprint/DataStruct/S_CharacterInfo Structure"))
  (set `self.CharacterInfo` CharacterInfo))

(fn `ShowBlood`
  (bind _returnvalue (`GameplayStatics.GetPlayerController` 0))
  (bind _bloodinfo (`self.GetBloodInfo`))
  (bind _wb_blood (`self.WB_Blood`))
  (set `self.IsBloodBarShowing` true)
  (`/Engine/EditorBlueprintResources/StandardMacros.IsValid` _wb_blood
    (:`Is Valid`
      (`Widget.SetVisibility` _wb_blood "Visible")
      (`/Game/UI/WB_Blood.SetBloodBarInfo` _wb_blood _bloodinfo))
    (:`Is Not Valid`
      (bind _returnvalue_2 (`|CreateWidget` "/Game/UI/WB_Blood.WB_Blood_C" _returnvalue))
      (`UserWidget.SetPositionInViewport` _returnvalue_2 (- (`GameplayStatics.ProjectWorldToScreen` _returnvalue (`self.K2_GetActorLocation`)) (100.0 500.0)) true)
      (`/Game/UI/WB_Blood.SetBloodBarInfo` _returnvalue_2 _bloodinfo)
      (`UserWidget.AddToViewport` _returnvalue_2 0)
      (set `self.WB_Blood` _returnvalue_2))))

(fn `ShowCharacterInfo`
  (bind _wb_targetactor (`/Game/UI/WB_Hud.WB_TargetActor` (`/Game/Blueprint/GameAPI_Lib.GetHudWidget`)))
  (`/Game/UI/WB_SelectedCrtInfo.SetCharacterInfo` _wb_targetactor (`self.CharacterInfo`))
  (`Widget.SetVisibility` _wb_targetactor "Visible"))

(fn `UpdateBloodBar`
  (bind _wb_blood (`self.WB_Blood`))
  (bind (_screenposition _returnvalue) (`GameplayStatics.ProjectWorldToScreen` (`GameplayStatics.GetPlayerController` 0) (+ (`self.K2_GetActorLocation`) (* (`.BoxExtent` (`KismetSystemLibrary.GetComponentBounds` (`self.Mesh`))) (0.0 0.0 1.0)))))
  (`/Engine/EditorBlueprintResources/StandardMacros.IsValid` _wb_blood
    (:`Is Valid`
      (if (`self.IsBloodBarShowing`)
        (`/Game/UI/WB_Blood.SetBloodBarInfo` _wb_blood (`self.GetBloodInfo`))
        (if _returnvalue
          (`UserWidget.SetPositionInViewport` _wb_blood (- _screenposition (70.0 0.0)) true)
          (else
            (`UserWidget.SetPositionInViewport` _wb_blood (-2000.0 0.0) true)))))))

(fn `UserConstructionScript`)