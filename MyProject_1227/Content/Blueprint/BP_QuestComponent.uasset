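; BP_QuestComponent is a quest log component that keeps separate arrays of open, solved and failed quests.
; Getters expose each array, and name checks loop through them comparing QuestName, overwriting the result each pass so only the last entry decides it.
; AddQuest adds a quest uniquely to the open array and prints its name.
; Nothing here moves quests into the solved or failed arrays, and Tick and BeginPlay are unused.
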(event EventTick
  (params (DeltaSeconds :type Float%20%28single-precision%29)))

(event EventBeginPlay)

(fn GetOpenQuests
  (return (Variables|Default|GetOpenQuests)))

(fn GetSolvedQuests
  (return (Variables|Default|GetSolvedQuests)))

(fn GetFailedQuests
  (return (Variables|Default|GetFailedQuests)))

(fn IsQuestOpenbyName
  (params (QuestNameToCheck :type Text))
  ;[1 1 1] Go through all the quests and look for a match
  (for _array_element (Variables|Default|GetOpenQuests)
    (if (Utilities|Enum|Equal(Enum) (Variables|/Game/Blueprint/Quest.Quest_C|GetQuestName _array_element) QuestNameToCheck)
      (LocalVariables|SetQuestIsOpen true)
      (else
        (LocalVariables|SetQuestIsOpen false))))
  (return (LocalVariables|GetQuestIsOpen)))

(fn IsQuestSolvedbyName
  (params (QuestNameToCheck :type Text))
  ;[1 1 1] Go through all the quests and look for a match
  (for _array_element (Variables|Default|GetSolvedQuests)
    (if (Utilities|Enum|Equal(Enum) (Variables|/Game/Blueprint/Quest.Quest_C|GetQuestName _array_element) QuestNameToCheck)
      (LocalVariables|SetQuestIsSolved true)
      (else
        (LocalVariables|SetQuestIsSolved false))))
  (return (LocalVariables|GetQuestIsSolved)))

(fn IsQuestFailedbyName
  (params (QuestNameToCheck :type Text))
  ;[1 1 1] Go through all the quests and look for a match
  (for _array_element (Variables|Default|GetFailedQuests)
    (if (Utilities|Enum|Equal(Enum) (Variables|/Game/Blueprint/Quest.Quest_C|GetQuestName _array_element) QuestNameToCheck)
      (LocalVariables|SetQuestIsFailed true)
      (else
        (LocalVariables|SetQuestIsFailed false))))
  (return (LocalVariables|GetQuestIsFailed)))

(fn AddQuest
  (params (NewQuest :type Quest%20Object%20Reference))
  ;[1 1 1] Add the quest to the array of open quests
  (Utilities|Array|AddUnique (Variables|Default|GetOpenQuests) NewQuest)
  (Development|PrintString (Utilities|String|Append "Received quest: " (Utilities|String|ToString(Text) (Variables|/Game/Blueprint/Quest.Quest_C|GetQuestName NewQuest)))))