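; GameAPI_Lib is a Blueprint function library of small gameplay helpers.
; GetCloseActor scans every actor of a given class and returns those within a radius of player 0's character.
; GetIntStringFromFloat turns a float into the text before its decimal point.
; GetHudWidget finds the first WB_Hud widget and returns it cast to that type.
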(fn GetCloseActor
  (params (Actor :type Actor%20Class%20Reference) (Radius :type Float%20%28single-precision%29))
  (bind _returnvalue (Game|GetPlayerCharacter 0))
  (bind _outactors (Actor|GetAllActorsOfClass _returnvalue Actor))
  (for _array_element _outactors
    (if (< (Math|Vector|VectorLength (- (Transformation|GetActorLocation _returnvalue) (Transformation|GetActorLocation _array_element))) Radius)
      (Utilities|Array|AddUnique (LocalVariables|GetOutActors) _array_element)))
  (return (LocalVariables|GetOutActors)))

(fn GetIntStringfromFloat
  (params (%20%20 :type Float%20%28single-precision%29))
  (bind _returnvalue (Utilities|String|ToString(Float) %20%20))
  (return (Utilities|String|Left _returnvalue (Utilities|String|FindSubstring _returnvalue "."))))

(fn GetHudWidget
  (bind _foundwidgets (Widget|GetAllWidgetsOfClass 0 "/Game/UI/WB_Hud.WB_Hud_C" false))
  (bind _aswb_hud (Utilities|Casting|CastToWB_Hud (Utilities|Array|Get(acopy) _foundwidgets))
    (:then
      _)
    (:CastFailed
      _))
  (return _aswb_hud))