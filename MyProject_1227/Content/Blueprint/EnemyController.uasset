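; AI controller for standard enemies that feeds sight, sound and alerts from other AI into a behavior tree through its blackboard.
; On begin play, after a short spawn delay, it converts the pawn's patrol points to world space, stores home location and attack range, then runs the tree.
; Seeing a pawn sets the attack target and reruns the tree; noises and alerts set an investigate location.
; A reset event clears both target and investigation.
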(event `ResetTarget`
  (bind _returnvalue (`AIBlueprintHelperLibrary.GetBlackboard` self))
  ;[1 1 1] Reset target to nothing
  (`KismetSystemLibrary.PrintString` "REset")
  (`self.UseBlackboard` "/Game/BehaviorTree/EnemyBlackboardData.EnemyBlackboardData")
  (`BlackboardComponent.SetValueAsObject` _returnvalue (`self.TargetToAttack`) null)
  (`BlackboardComponent.SetValueAsBool` _returnvalue (`self.HasInvestigateLocation`) false))

(event `self.ReceiveBeginPlay`
  (bind _returnvalue (`self.K2_GetPawn`))
  (bind _returnvalue_2 (`AIBlueprintHelperLibrary.GetBlackboard` self))
  ;[1 1 1] Delay until pawn is spawned
  (`KismetSystemLibrary.Delay` 0.2)
  (bind _asstandard_enemy (cast `/Game/Blueprint/StandardEnemy` _returnvalue))
  ;[1 1 1] Get patrol points and convert them to world space
  (for _array_element (`/Game/Blueprint/StandardEnemy.PatrolPoints` _asstandard_enemy)
    (`KismetArrayLibrary.Array_Add` (`self.PatrolPoints`) (`KismetMathLibrary.TransformLocation` (`self.GetTransform` _asstandard_enemy) _array_element)))
  (bind _attackrange (`/Game/Blueprint/StandardEnemy.GetAttackRange` _asstandard_enemy))
  (set `self.AttackRangeValue` _attackrange)
  ;[1 1 1] Keep track where the Enemy started so he can return to this position and get the control points
  (`self.UseBlackboard` "/Game/BehaviorTree/EnemyBlackboardData.EnemyBlackboardData")
  (`BlackboardComponent.SetValueAsVector` _returnvalue_2 (`self.HomeLocation`) (`self.K2_GetActorLocation` _returnvalue))
  (`BlackboardComponent.SetValueAsFloat` _returnvalue_2 (`self.AttackRange`) (`self.AttackRangeValue`))
  (`self.RunBehaviorTree` "/Game/BehaviorTree/EnemyBehaviourTree.EnemyBehaviourTree"))

(event `self.PawnSensing1.OnSeePawn`
  (params (Pawn :type "Pawn Object Reference"))
  (bind _returnvalue (`AIBlueprintHelperLibrary.GetBlackboard` self))
  ;[1 1 1] Let the behaviour tree know that we see the player and want to attack him
  (`self.UseBlackboard` "/Game/BehaviorTree/EnemyBlackboardData.EnemyBlackboardData")
  (`BlackboardComponent.SetValueAsVector` _returnvalue (`self.TargetLocation`) (`self.K2_GetActorLocation` Pawn))
  (`BlackboardComponent.SetValueAsObject` _returnvalue (`self.TargetToAttack`) Pawn)
  (`self.RunBehaviorTree` "/Game/BehaviorTree/EnemyBehaviourTree.EnemyBehaviourTree"))

(event `self.PawnSensing1.OnHearNoise`
  (params (Instigator :type "Pawn Object Reference") (Location :type "Vector Structure (by ref)") (Volume :type "Float (single-precision)"))
  (bind _returnvalue (`AIBlueprintHelperLibrary.GetBlackboard` self))
  ;[1 1 1] If the AI hears something, make it go there
  (`self.UseBlackboard` "/Game/BehaviorTree/EnemyBlackboardData.EnemyBlackboardData")
  (`BlackboardComponent.SetValueAsVector` _returnvalue (`self.InvestigateLocation`) Location)
  (`BlackboardComponent.SetValueAsBool` _returnvalue (`self.HasInvestigateLocation`) true))

(event `/Game/Blueprint/Interface/BPI_EnemyController.AlertOthers`
  (params (LocationOfInterest :type "Vector Structure"))
  (bind _returnvalue (`AIBlueprintHelperLibrary.GetBlackboard` self))
  ;[1 1 1] If alerted by another AI make it investigate that location
  (`self.UseBlackboard` "/Game/BehaviorTree/EnemyBlackboardData.EnemyBlackboardData")
  (`BlackboardComponent.SetValueAsVector` _returnvalue (`self.InvestigateLocation`) LocationOfInterest)
  (`BlackboardComponent.SetValueAsBool` _returnvalue (`self.HasInvestigateLocation`) true))

(fn `UserConstructionScript`)