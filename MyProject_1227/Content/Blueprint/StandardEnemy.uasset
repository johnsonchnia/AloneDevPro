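; Standard enemy character for an RPG that can be targeted, attacks the player and awards XP when killed.
; Attack plays a montage and immediately damages player 0, with no range or block check of its own.
; HitEnemy subtracts health or calls Die, notifies the killer and returns the blocking state.
; Death ragdolls the mesh, removes the capsule and destroys the actor after a delay; GetHealth and GetMana only return zero.
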(event EventDie
  ;[1 1 1] Death
  (Variables|Default|SetIsDead true)
  (Physics|SetSimulatePhysics (Variables|Character|GetMesh) true)
  (Components|DestroyComponent (Variables|Collision|GetCapsuleComponent))
  (Components|DestroyComponent)
  (Utilities|FlowControl|Delay 5.0)
  (Actor|DestroyActor))

(event EventSetActiveTarget
  (params (bIsTargeted :type Boolean))
  ;[1 1 1] Enemy gets targeted by player / or ends the target
  (Rendering|SetVisibility bIsTargeted false))

(fn ConstructionScript
  (Variables|/Script/Engine.CharacterMovementComponent|SetMaxWalkSpeed (Variables|Character|GetCharacterMovement) (Variables|EnemyBehaviour|GetEnemySpeed)))

(fn Attack
  ;[1 1 1] Cant attack when dead
  (if (not (Variables|Default|GetIsDead))
    ;[1 1 1] Play attack animation
    (Animation|PlayAnimMontage (Variables|Default|GetAttackMontage) 1.0 "None")
    ;[1 1 1] Do damage depending on wether player blocks the attack or not
    (bind _asrpgcharacter (Utilities|Casting|CastToRPGCharacter (Game|GetPlayerCharacter 0)))
    (Default|TakeDamage _asrpgcharacter (Variables|Enemy|GetDamage))))

(fn GetHealth
  (return 0.0))

(fn GetAttackRange
  ;[1 1 1] Return the attack range of this enemy
  (return (Variables|Default|GetAttackRange)))

(fn GetMana
  (return 0.0))

(fn HitEnemy
  (params (Damage :type Float%20%28single-precision%29) (Instigator :type Actor%20Object%20Reference))
  ;[1 1 1] Cache value
  (LocalVariables|SetDamageTaken Damage)
  ;[1 1 1] Decide wether enemy dies or takes damage
  (if (> (- (Variables|Enemy|GetHealth) (LocalVariables|GetDamageTaken)) 0.0)
    ;[1 1 1] Inflict damage
    (Variables|Enemy|SetHealth (- (Variables|Enemy|GetHealth) (LocalVariables|GetDamageTaken)))
    (else
      ;[1 1 1] Enemy gets killed, let player know
      (CallFunction|Die)
      (bind _asrpgcharacter (Utilities|Casting|CastToRPGCharacter Instigator))
      (Default|HasKilledSomeone _asrpgcharacter self)
      (Default|AwardXP _asrpgcharacter (Variables|Enemy|GetXPToGive))))
  (return (Variables|Default|GetIsBlocking)))